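; Markimoo is the player's Paper2D side-scrolling character, handling movement, jumping, punching and HUD widget creation.
; An enum state selects sprite flipbooks, with CanMove gating movement and briefly locking during punches.
; Interact dispatches on note type to close or replace note boxes, including a wolf warning.
; StartFight creates a Dodgebar and runs one reaction-timer update; F sets dodging, and key 1 flashes a test jumpscare.
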(event `self.ReceiveBeginPlay`
  ;[1 1 1] Event Begin on play
  (set `self.enum_state` "NewEnumerator1")
  (set `self.enum_mode` "NewEnumerator2")
  (bind _returnvalue (`|CreateWidget` "/Game/NPOTG/Blueprints/Widgets/Admin_Widget.Admin_Widget_C"))
  (`UserWidget.AddToViewport` _returnvalue 0)
  (bind _returnvalue_2 (`|CreateWidget` "/Game/NPOTG/Blueprints/Widgets/Lifebar.Lifebar_C"))
  (set `self.lifebar` _returnvalue_2)
  (`UserWidget.AddToViewport` _returnvalue_2 0)
  (bind _returnvalue_3 (`|CreateWidget` "/Game/NPOTG/Blueprints/Widgets/SKillbar.SKillbar_C"))
  (`UserWidget.AddToViewport` _returnvalue_3 0)
  (`ActorComponent.SetIsReplicated` (`self.Sprite`) true))

(event `UpdateAnimation`
  (bind _sprite (`self.Sprite`))
  ;[1 1 1] Handle Animation
  (switch `/Game/NPOTG/Blueprints/Enumeration/Marki-State` (`self.enum_state`)
    (:`NewEnumerator1`
      (`PaperFlipbookComponent.SetFlipbook` _sprite (select `bool` (> (`KismetMathLibrary.VSize` (`self.GetVelocity`)) 0.0) :`false` "/Game/NPOTG/Sprites/Charaktere/HEro_guy/hauptcharakter_mittelalter_standing.hauptcharakter_mittelalter_standing" :`true` "/Game/NPOTG/Sprites/Charaktere/HEro_guy/Hauptcharakter_mittelalter_walking.Hauptcharakter_mittelalter_walking" :!type "PaperFlipbook Object Reference") :!label _label))
    (:`NewEnumerator2`
      (goto _label))
    (:`NewEnumerator3`
      (`PaperFlipbookComponent.SetFlipbook` _sprite "/Game/NPOTG/Sprites/Charaktere/HEro_guy/hauptcharakter_mittelater_jump.hauptcharakter_mittelater_jump"))
    (:`NewEnumerator4`
      (set `self.wolfcanmove` false))
    (:`NewEnumerator7`
      (`PaperFlipbookComponent.SetFlipbook` _sprite "/Game/NPOTG/Sprites/Charaktere/HEro_guy/hauptcharakter_mittelalter_slashing.hauptcharakter_mittelalter_slashing"))))

(event `InputAxis|MoveRight`
  (params (AxisValue :type "Float (single-precision)"))
  ;[1 1 1] Handle movement
  (if (`self.can_move`)
    (`self.AddMovementInput` (1.0 0.0 0.0) AxisValue)
    (`self.UpdateAnimation`)
    (`/Engine/EditorBlueprintResources/StandardMacros.CompareFloat` AxisValue
      (:`>`
        (`Controller.SetControlRotation` (`self.GetController`) (`KismetMathLibrary.MakeRot` 0.0 0.0))
        (set `self.Direction` 1.0))
      (:`<`
        (`Controller.SetControlRotation` (`self.GetController`) (`KismetMathLibrary.MakeRot` 0.0 180.0))
        (set `self.Direction` -1.0)))
    (else
      (`self.UpdateAnimation`))))

(event `Key|Escape`
  (:`Pressed`
    (`KismetSystemLibrary.QuitGame` null "Quit")))

(event `InputAction|Jump`
  ;[1 1 1] Handle Jump
  (:`Pressed`
    (if (not (`self.jumping`))
      (set `self.jumping` true)
      (if (`self.can_move`) :!label _label_2
        (`self.Jump`)
        (set `self.enum_state` "NewEnumerator3"))))
  (:`Released`
    (`self.StopJumping` :!label _label_3)))

(event `InputAction|Punch`
  ;[1 1 1] Handle Punch
  (:`Pressed`
    (if (`self.can_move`)
      (`self.AddMovementInput` (0.5 0.0 0.0) (* (`self.Direction`) 1.0))
      (set `self.enum_state` "NewEnumerator7")
      (set `self.can_move` false)
      (`KismetSystemLibrary.Delay` 0.5)
      (set `self.can_move` true)
      (set `self.enum_state` "NewEnumerator1"))))

(event `InputTouch`
  (params (Location :type "Vector Structure") (FingerIndex :type "ETouchIndex Enum"))
  ;[1 1 1] Handle Jump
  (:`Pressed`
    (goto _label_2))
  (:`Released`
    (goto _label_3)))

(event `self.OnLanded`
  (params (Hit :type "HitResult Structure (by ref)"))
  ;[1 1 1] Handle Jump
  (set `self.jumping` false)
  (set `self.enum_state` "NewEnumerator1"))

(event `self.ReceiveHit`
  (params (MyComp :type "PrimitiveComponent Object Reference") (Other :type "Actor Object Reference") (OtherComp :type "PrimitiveComponent Object Reference") (bSelfMoved :type Boolean) (HitLocation :type "Vector Structure") (HitNormal :type "Vector Structure") (NormalImpulse :type "Vector Structure") (Hit :type "HitResult Structure (by ref)"))
  (set `self.jumping` false))

(event `InputAction|Interact`
  ;[1 1 1] Handle Interact
  (:`Pressed`
    (bind _interaxcttype (`self.GetInteractType`))
    (`self.Interact` _interaxcttype)))

(event `Key|One`
  ;[1 1 1] Test Jumpscare
  (:`Pressed`
    (`self.DisableInput` (`GameplayStatics.GetPlayerController` 0) null)
    (bind _returnvalue (`|CreateWidget` "/Game/NPOTG/Blueprints/Widgets/Horrorscreen.Horrorscreen_C"))
    (`UserWidget.AddToViewport` _returnvalue 0)
    (`KismetSystemLibrary.Delay` 0.2)
    (bind _foundwidgets (`WidgetBlueprintLibrary.GetAllWidgetsOfClass` "/Game/NPOTG/Blueprints/Widgets/Horrorscreen.Horrorscreen_C"))
    (for _array_element _foundwidgets
      (`Widget.RemoveFromParent` _array_element))))

(event `Key|F`
  (:`Pressed`
    (set `self.enum_state` "NewEnumerator6"))
  (:`Released`
    (set `self.enum_state` "NewEnumerator1")))

(fn `gameOver`
  (`KismetSystemLibrary.QuitGame` null "Quit"))

(fn `GetInteractType`
  (returns (InteraxctType :type "/Game/NPOTG/Blueprints/Enumeration/InteractType Enum"))
  (return (`self.InteractType`)))

(fn `Interact`
  (params (Type :type "/Game/NPOTG/Blueprints/Enumeration/InteractType Enum"))
  (switch `/Game/NPOTG/Blueprints/Enumeration/InteractType` Type
    (:`NewEnumerator0`
      (bind _foundwidgets (`WidgetBlueprintLibrary.GetAllWidgetsOfClass` "/Game/NPOTG/Blueprints/Widgets/Notebox_empty.Notebox_empty_C"))
      (for _array_element _foundwidgets
        (`Widget.RemoveFromParent` _array_element)
        (set `self.can_move` true)))
    (:`NewEnumerator2`
      (`self.NotPartOfTheGameSequece`)
      (bind _foundwidgets_2 (`WidgetBlueprintLibrary.GetAllWidgetsOfClass` "/Game/NPOTG/Blueprints/Widgets/Notebox_empty.Notebox_empty_C"))
      (for _array_element_2 _foundwidgets_2
        (`Widget.RemoveFromParent` _array_element_2)
        (set `self.lifebar_rauschen` true)
        (bind _returnvalue (`|CreateWidget` "/Game/NPOTG/Blueprints/Widgets/Notebox_empty.Notebox_empty_C"))
        (set `/Game/NPOTG/Blueprints/Widgets/Notebox_empty.Is_Closeable` true _returnvalue)
        (set `/Game/NPOTG/Blueprints/Widgets/Notebox_empty.TextInhalt` "TAKE CARE WOLVES KILL YOU! Dodge their attacks in the green zone." _returnvalue)
        (set `/Game/NPOTG/Blueprints/Widgets/Notebox_empty.Textfarbe` (struct :`R` 0.38 :`G` 0.015022 :`B` 0.02591 :`A` 1.0) _returnvalue)
        (`self.SetInteractType` "NewEnumerator0")
        (`UserWidget.AddToViewport` _returnvalue 0)))))

(fn `NotPartOfTheGameSequece`)

(fn `Prepare_for_react`
  (set `self.Current_Reaktion_TIme` (`self.Max_Reaction_Time`)))

(fn `REACT!`
  (if (> (`self.Current_Reaktion_TIme`) 0.0)
    (bind _output_get (set `self.Current_Reaktion_TIme` (- (`self.Current_Reaktion_TIme`) (* (`GameplayStatics.GetWorldDeltaSeconds`) (`self.Reaktion_Time_dealy`)))))
    (bind _output_get_2 (set `/Game/NPOTG/Blueprints/Widgets/Dodgebar.Timer-percentage` (/ _output_get (`self.Max_Reaction_Time`)) (`self.Dodgebar`)))
    (if (== _output_get_2 0.0)
      (bind _foundwidgets (`WidgetBlueprintLibrary.GetAllWidgetsOfClass` "/Game/NPOTG/Blueprints/Widgets/Dodgebar.Dodgebar_C"))
      (for _array_element _foundwidgets
        (`Widget.RemoveFromParent` _array_element)
        (set `self.can_move` true)))
    (else
      (set `self.won_react` false))))

(fn `SetInteractType`
  (params (InteractType :type "/Game/NPOTG/Blueprints/Enumeration/InteractType Enum"))
  (set `self.InteractType` InteractType))

(fn `start fight`
  (bind _returnvalue (`|CreateWidget` "/Game/NPOTG/Blueprints/Widgets/Dodgebar.Dodgebar_C"))
  (set `self.Dodgebar` _returnvalue)
  (`UserWidget.AddToViewport` _returnvalue 0)
  (`self.Prepare_for_react`)
  (`self.REACT!`))

(fn `UserConstructionScript`)