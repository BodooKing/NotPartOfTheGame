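; Wolf enemy that starts a fight with the Markimoo player character when it enters the SeeCone.
; The cone overlap flags the sighting, sets Markimoo's state to SeenByWolf and calls StartFight.
; The wolf destroys itself when touched by a slashing Markimoo, or on Tick after a sighting once Markimoo's DefeatedEnemy is set.
; A timeline patrol between PointA and PointB exists but never runs.
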(event `self.ReceiveTick`
  (params (DeltaSeconds :type "Float (single-precision)"))
  (if (`self.sehe markimoo`)
    (bind _asmarkimoo (cast `/Game/NPOTG/Blueprints/Charaktere/Markimoo` (`GameplayStatics.GetPlayerCharacter` 0)))
    (if (`/Game/NPOTG/Blueprints/Charaktere/Markimoo.defeated enemy` _asmarkimoo)
      (`self.K2_DestroyActor`))))

(event `self.ReceiveActorBeginOverlap`
  (params (OtherActor :type "Actor Object Reference"))
  (bind _asmarkimoo (cast `/Game/NPOTG/Blueprints/Charaktere/Markimoo` (stale `self.ReceiveHit` Other) :!label _label))
  (switch `/Game/NPOTG/Blueprints/Enumeration/Marki-State` (`/Game/NPOTG/Blueprints/Charaktere/Markimoo.enum_state` _asmarkimoo)
    (:`NewEnumerator7`
      (`self.K2_DestroyActor`))))

(event `self.ReceiveHit`
  (params (MyComp :type "PrimitiveComponent Object Reference") (Other :type "Actor Object Reference") (OtherComp :type "PrimitiveComponent Object Reference") (bSelfMoved :type Boolean) (HitLocation :type "Vector Structure") (HitNormal :type "Vector Structure") (NormalImpulse :type "Vector Structure") (Hit :type "HitResult Structure (by ref)"))
  (goto _label))

(event `self.see cone.OnComponentBeginOverlap`
  (params (OtherActor :type "Actor Object Reference") (OtherComp :type "PrimitiveComponent Object Reference") (OtherBodyIndex :type Integer) (bFromSweep :type Boolean) (SweepResult :type "HitResult Structure (by ref)"))
  (set `self.sehe markimoo` true)
  (bind _asmarkimoo (cast `/Game/NPOTG/Blueprints/Charaktere/Markimoo` OtherActor))
  (set `/Game/NPOTG/Blueprints/Charaktere/Markimoo.enum_state` "NewEnumerator4" _asmarkimoo)
  (`/Game/NPOTG/Blueprints/Charaktere/Markimoo.start fight` _asmarkimoo))

(fn `UserConstructionScript`)