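; Questdude is a quest-giver NPC that hands the player a quest to kill all wolves.
; The first time Capsule1 registers an overlap, it freezes the Markimoo player's movement and shows the quest text in a closeable Notebox_empty widget.
; It then sets the player's interact type, marks itself finished so it does not repeat, and adds the HUDQUESTKILLALL widget to the viewport.
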(event `self.Capsule1.OnComponentBeginOverlap`
  (params (OtherActor :type "Actor Object Reference") (OtherComp :type "PrimitiveComponent Object Reference") (OtherBodyIndex :type Integer) (bFromSweep :type Boolean) (SweepResult :type "HitResult Structure (by ref)"))
  (bind _returnvalue (`GameplayStatics.GetPlayerCharacter` 0))
  (if (not (`self.prozedure finished`))
    (bind _returnvalue_2 (`|CreateWidget` "/Game/NPOTG/Blueprints/Widgets/Notebox_empty.Notebox_empty_C"))
    (bind _asmarkimoo (cast `/Game/NPOTG/Blueprints/Charaktere/Markimoo` _returnvalue))
    (set `/Game/NPOTG/Blueprints/Charaktere/Markimoo.can_move` false _asmarkimoo)
    (set `/Game/NPOTG/Blueprints/Widgets/Notebox_empty.TextInhalt` "Hello strong goodlooking manly Warrior! Only you can help me because you have a sword! Kill all wolves please. They are kinda annoying." _returnvalue_2)
    (set `/Game/NPOTG/Blueprints/Widgets/Notebox_empty.Is_Closeable` true _returnvalue_2)
    (`UserWidget.AddToViewport` _returnvalue_2 0)
    (bind _asmarkimoo_2 (cast `/Game/NPOTG/Blueprints/Charaktere/Markimoo` _returnvalue))
    (`/Game/NPOTG/Blueprints/Charaktere/Markimoo.SetInteractType` _asmarkimoo_2 "NewEnumerator0")
    (set `self.prozedure finished` true)
    (bind _returnvalue_3 (`|CreateWidget` "/Game/NPOTG/Blueprints/Widgets/HUD-QUEST-KILLALL.HUD-QUEST-KILLALL_C"))
    (`UserWidget.AddToViewport` _returnvalue_3 0)))

(fn `UserConstructionScript`)