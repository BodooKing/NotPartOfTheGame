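; Door Blueprint that swaps its sprite between open and closed as something enters or leaves its capsule trigger.
; Each begin overlap shows the open sprite and toggles the MarkimooInVillage boolean, apparently tracking whether Markimoo is inside the village.
; End overlap restores the closed sprite.
; The overlapping actor is not checked, so any overlap triggers both the visual change and the toggle.
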(event `self.Capsule1.OnComponentBeginOverlap`
  (params (OtherActor :type "Actor Object Reference") (OtherComp :type "PrimitiveComponent Object Reference") (OtherBodyIndex :type Integer) (bFromSweep :type Boolean) (SweepResult :type "HitResult Structure (by ref)"))
  (`PaperSpriteComponent.SetSprite` (`self.PaperSprite1`) "/Game/NPOTG/Sprites/Tiles/door_open_Sprite.door_open_Sprite")
  (if (`self.markimoo in village`)
    (set `self.markimoo in village` false)
    (else
      (set `self.markimoo in village` true))))

(event `self.Capsule1.OnComponentEndOverlap`
  (params (OtherActor :type "Actor Object Reference") (OtherComp :type "PrimitiveComponent Object Reference") (OtherBodyIndex :type Integer))
  (`PaperSpriteComponent.SetSprite` (`self.PaperSprite1`) "/Game/NPOTG/Sprites/Tiles/door_closed_Sprite.door_closed_Sprite"))

(fn `UserConstructionScript`)