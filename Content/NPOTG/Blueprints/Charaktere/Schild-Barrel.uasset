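; Sign Blueprint for the storage place that shows a one-time note warning players not to smash the barrels with swords.
; The first overlap with Capsule1, by any actor, creates a closeable Notebox_empty widget with hardcoded text.
; It disables movement on the Markimoo player, sets its interact type and latches ProzedureFinished against repeats.
; Movement is not restored in this Blueprint.
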(event `self.Capsule1.OnComponentBeginOverlap`
  (params (OtherActor :type "Actor Object Reference") (OtherComp :type "PrimitiveComponent Object Reference") (OtherBodyIndex :type Integer) (bFromSweep :type Boolean) (SweepResult :type "HitResult Structure (by ref)"))
  (bind _returnvalue (`GameplayStatics.GetPlayerCharacter` 0))
  (if (not (`self.prozedure finished`))
    (bind _returnvalue_2 (`|CreateWidget` "/Game/NPOTG/Blueprints/Widgets/Notebox_empty.Notebox_empty_C"))
    (set `/Game/NPOTG/Blueprints/Widgets/Notebox_empty.Is_Closeable` true _returnvalue_2)
    (set `/Game/NPOTG/Blueprints/Widgets/Notebox_empty.TextInhalt` "Welcome to the Storage Place! The following Note is for the Adventurers out there: DO NOT DESTROY THE BARRELS WITH YOUR SWORDS! You dont get anything from that." _returnvalue_2)
    (bind _asmarkimoo (cast `/Game/NPOTG/Blueprints/Charaktere/Markimoo` _returnvalue))
    (set `/Game/NPOTG/Blueprints/Charaktere/Markimoo.can_move` false _asmarkimoo)
    (`UserWidget.AddToViewport` _returnvalue_2 0)
    (bind _asmarkimoo_2 (cast `/Game/NPOTG/Blueprints/Charaktere/Markimoo` _returnvalue))
    (`/Game/NPOTG/Blueprints/Charaktere/Markimoo.SetInteractType` _asmarkimoo_2 "NewEnumerator0")
    (set `self.prozedure finished` true)))

(fn `UserConstructionScript`)